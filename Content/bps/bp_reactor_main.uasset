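; Main reactor Blueprint that tracks power, fuel and water, and decides when the player is fired or the reactor explodes.
; It totals power and fuel from active, placed entries in Bp_fuel after a startup delay and on a recalculate event.
; Tick flags out-of-range power as fired, otherwise drains water, showing a low-water warning, reducing power when overfilled and flagging an explosion when empty.
; Both endings currently only print a message once.
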(event `self.ReceiveBeginPlay`
  (bind _returnvalue (`GameplayStatics.GetActorOfClass` "/Game/bps/bp_fuel.bp_fuel_C"))
  (set `self.BP_fuel` _returnvalue)
  (`KismetSystemLibrary.Delay` 1.0)
  (set `self.tmp_power` 0.0)
  (set `self.tmp_fuel` 0.0)
  (for _array_element (`/Game/bps/bp_fuel.fuels` (`self.BP_fuel`))
    (if (and (`.active_9_DDA82008483E56247C1AD5A378F9DDC9` (break `/Game/structures/S_fuel` _array_element)) (`.placed_11_29C937AC410BF15DBEE16DB8BDA8F6FA` (break `/Game/structures/S_fuel` _array_element)))
      (set `self.tmp_power` (+ 100.0 (`self.tmp_power`)))
      (set `self.tmp_fuel` (+ (`.Fuel_5_EA564127436107125587148396CBF3D6` (break `/Game/structures/S_fuel` _array_element)) (`self.tmp_fuel`)))))
  (set `self.fuel` (`self.tmp_fuel`))
  (set `self.power` (`self.tmp_power`)))

(event `ED_Recalculate_Power_Event`
  (set `self.tmp_power` 0.0)
  (set `self.tmp_fuel` 0.0)
  (for _array_element (`/Game/bps/bp_fuel.fuels` (`self.BP_fuel`))
    (if (and (`.active_9_DDA82008483E56247C1AD5A378F9DDC9` (break `/Game/structures/S_fuel` _array_element)) (`.placed_11_29C937AC410BF15DBEE16DB8BDA8F6FA` (break `/Game/structures/S_fuel` _array_element)))
      (set `self.tmp_power` (+ 100.0 (`self.tmp_power`)))
      (set `self.tmp_fuel` (+ (`.Fuel_5_EA564127436107125587148396CBF3D6` (break `/Game/structures/S_fuel` _array_element)) (`self.tmp_fuel`)))))
  (set `self.power` (`self.tmp_power`))
  (set `self.fuel` (`self.tmp_fuel`)))

(event `self.ReceiveTick`
  (params (DeltaSeconds :type "Float (single-precision)"))
  (bind _plane_water_warning (`self.plane_water_warning`))
  (if (or (> (`self.power`) (`self.max_power`)) (< (`self.power`) (`self.min_power`)))
    (set `self.get_fired` true))
  (if (`self.get_fired`)
    (`/Engine/EditorBlueprintResources/StandardMacros.DoOnce` false
      (:`Completed`
        (`KismetSystemLibrary.PrintString` "Fired")))
    (elif (`self.boom`)
      (`/Engine/EditorBlueprintResources/StandardMacros.DoOnce` false
        (:`Completed`
          (`KismetSystemLibrary.PrintString` "Boom")))
      (else
        (set `self.water` (- (`self.water`) (`self.water_fall_rate`)))
        (if (< (`self.water`) 10.0)
          (`SceneComponent.SetVisibility` _plane_water_warning true false)
          (else
            (`SceneComponent.SetVisibility` _plane_water_warning false false)))
        (if (<= (`self.water`) 0.0)
          (set `self.boom` true))
        (if (> (`self.water`) 100.0)
          (set `self.power` (- (`self.power`) 0.1)))))))

(fn `UserConstructionScript`)