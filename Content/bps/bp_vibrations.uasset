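; Reactor vibration-matching minigame in which the player nudges their vibration up or down to match a drifting target.
; Tick runs a state machine that waits a random delay, lerps the target to a new random value, then waits for a near match.
; A match snaps the player's value to the target and briefly locks input.
; Both values drive sine wave amplitude and frequency through separate Material Parameter Collections.
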(event `self.ReceiveBeginPlay`
  (`self.set_current_vibration` 50.0)
  (`self.set_target_vibration` 50.0)
  (set `self.target_change_wait_delay` "0001.01.01-00.00.00"))

(event `self.ReceiveTick`
  (params (DeltaSeconds :type "Float (single-precision)"))
  (`self.increment_player_vibration_if_active`)
  (`self.perform_wait_for_change`)
  (`self.perform_move_to_target_destination`)
  (`self.perform_wait_for_fix`))

(event `ButtonSelectionDispatcher_Event`
  (bind _holding_component (`self.holding_component`))
  (if (`KismetStringLibrary.EqualEqual_StrStr` _holding_component "Up")
    (set `self.increment_direction` 0.5)
    (elif (`KismetStringLibrary.EqualEqual_StrStr` _holding_component "Down")
      (set `self.increment_direction` -0.5))))

(fn `calculate_wave_params`
  (params (Vibration :type "Float (double-precision)"))
  (returns (Amplitude :type "Float (double-precision)") (Frequency :type "Float (double-precision)"))
  (return (+ (/ Vibration 200.0) 0.1) (+ (/ Vibration 20.0) 1.0)))

(fn `get_time_in_x_seconds`
  (params (Seconds :type "Float (single-precision)"))
  (returns (ReturnValue :type "DateTime Structure"))
  (return (+ (`KismetMathLibrary.Now`) (`KismetMathLibrary.FromSeconds` Seconds))))

(fn `has_happened`
  (params (Time :type "DateTime Structure"))
  (returns (ReturnValue :type Boolean))
  (return (<= Time (`KismetMathLibrary.Now`))))

(fn `increment_player_vibration_if_active`
  (if (`self.active`)
    (bind _returnvalue (`self.has_happened` (`self.input_delay`)))
    (if _returnvalue
      (`self.set_current_vibration` (`KismetMathLibrary.FClamp` (+ (`self.current_vibration`) (`self.increment_direction`)) 0.0 100.0)))))

(fn `perform_move_to_target_destination`
  (if (`|EnumEquality` (`self.vibration_change_state`) "NewEnumerator1")
    (bind _output_get (set `self.target_change_move_progress` (`KismetMathLibrary.FClamp` (+ (`self.target_change_move_progress`) 0.001))))
    (`self.set_target_vibration` (`KismetMathLibrary.Lerp` (`self.target_change_start`) (`self.target_change_destination`) _output_get))
    (if (== (`self.target_change_move_progress`) 1.0)
      (set `self.vibration_change_state` "NewEnumerator2")
      (`KismetSystemLibrary.PrintString` "Finished moving to target vibration"))))

(fn `perform_wait_for_change`
  (if (`|EnumEquality` (`self.vibration_change_state`) "NewEnumerator0")
    (bind _returnvalue (`self.has_happened` (`self.target_change_wait_delay`)))
    (if _returnvalue
      (set `self.target_change_start` (`self.target_vibration`))
      (bind _output_get (set `self.target_change_destination` (`KismetMathLibrary.RandomFloatInRange` 0.0 100.0)))
      (set `self.target_change_move_progress` 0.0)
      (set `self.vibration_change_state` "NewEnumerator1")
      (`KismetSystemLibrary.PrintString` (`KismetStringLibrary.Concat_StrStr` "Finished waiting for change, new target:" (`KismetStringLibrary.Conv_DoubleToString` _output_get))))))

(fn `perform_wait_for_fix`
  (bind _returnvalue (`KismetMathLibrary.RandomFloatInRange` 500.0 1000.0))
  (bind _returnvalue_2 (`KismetMathLibrary.Abs` (- (`self.target_vibration`) (`self.current_vibration`))))
  (if (`|EnumEquality` (`self.vibration_change_state`) "NewEnumerator2")
    (if (<= _returnvalue_2 2.0)
      (`self.set_current_vibration` (`self.target_vibration`))
      (bind _returnvalue_3 (`self.get_time_in_x_seconds` _returnvalue))
      (set `self.target_change_wait_delay` _returnvalue_3)
      (set `self.vibration_change_state` "NewEnumerator0")
      (bind _returnvalue_4 (`self.get_time_in_x_seconds` 3.0))
      (set `self.input_delay` _returnvalue_4)
      (`KismetSystemLibrary.PrintString` (`KismetStringLibrary.Concat_StrStr` "Player fixed vibration with difference:" (`KismetStringLibrary.Conv_DoubleToString` _returnvalue_2)))
      (`KismetSystemLibrary.PrintString` (`KismetStringLibrary.Concat_StrStr` "Delay for: " (`KismetStringLibrary.Conv_DoubleToString` _returnvalue))))))

(fn `set_current_vibration`
  (params (current_fibration :type "Float (double-precision)"))
  (bind _output_get (set `self.current_vibration` current_fibration))
  (bind (_amplitude _frequency) (`self.calculate_wave_params` _output_get))
  (`KismetMaterialLibrary.SetScalarParameterValue` "/Game/mats/player_sine_mpc.player_sine_mpc" "Amplitude" _amplitude)
  (`KismetMaterialLibrary.SetScalarParameterValue` "/Game/mats/player_sine_mpc.player_sine_mpc" "Frequency" _frequency))

(fn `set_target_vibration`
  (params (target_vibration :type "Float (double-precision)"))
  (bind _output_get (set `self.target_vibration` target_vibration))
  (bind (_amplitude _frequency) (`self.calculate_wave_params` _output_get))
  (`KismetMaterialLibrary.SetScalarParameterValue` "/Game/mats/reactor_sine_mpc.reactor_sine_mpc" "Amplitude" _amplitude)
  (`KismetMaterialLibrary.SetScalarParameterValue` "/Game/mats/reactor_sine_mpc.reactor_sine_mpc" "Frequency" _frequency))

(fn `UserConstructionScript`)