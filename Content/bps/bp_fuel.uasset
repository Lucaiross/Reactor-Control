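; Fuel manager for the reactor that spawns a 3x3 grid of green physics cubes, tracked in the Fuels struct array and tagged with their array index.
; A repeating delayed event turns a random cell red and empties it.
; The Cube trigger destroys an overlapping cell and spawns a fresh one.
; Cube1 overlaps set placed state via tags, and both placement changes and depletion make Bp_reactor_main recalculate power.
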(event `self.ReceiveBeginPlay`
  (bind (_returnvalue_x _returnvalue_y _returnvalue_z) (`KismetMathLibrary.BreakVector` (`SceneComponent.K2_GetComponentLocation` (`self.DefaultSceneRoot`))))
  (bind _returnvalue (`GameplayStatics.GetActorOfClass` "/Game/bps/bp_reactor_main.bp_reactor_main_C"))
  (set `self.Bp_reactor_main` _returnvalue)
  (for _index (range 3)
    (for _index_2 (range 3)
      (bind _returnvalue_2 (+ _returnvalue_x (`KismetMathLibrary.Conv_IntToDouble` (* _index_2 100))))
      (bind _returnvalue_3 (`AddComponent|NODE_AddStaticMeshComponent-0` :`RelativeTransform` (`KismetMathLibrary.MakeTransform` (`KismetMathLibrary.MakeVector` _returnvalue_2) (struct) (0.5 0.5 0.5))))
      (`SceneComponent.K2_SetWorldLocation` _returnvalue_3 (`KismetMathLibrary.MakeVector` _returnvalue_2 (+ _returnvalue_y (`KismetMathLibrary.Conv_IntToDouble` (* _index 100))) _returnvalue_z) false false)
      (`StaticMeshComponent.SetStaticMesh` _returnvalue_3 "/Engine/BasicShapes/Cube.Cube")
      (`PrimitiveComponent.SetSimulatePhysics` _returnvalue_3 true)
      (`PrimitiveComponent.SetMaterial` _returnvalue_3 0 "/AnimationSharing/AnimSharingGreen.AnimSharingGreen")
      (bind _returnvalue_4 (`KismetArrayLibrary.Array_Add` (`self.Fuels`) (make `/Game/structures/S_fuel` _returnvalue_3 100.0 true)))
      (bind _output_get (set `self.ind` (`KismetStringLibrary.Conv_IntToString` _returnvalue_4)))
      (bind _output_get_2 (set `self.tag` (`KismetStringLibrary.Conv_StringToName` _output_get)))
      (set `ActorComponent.ComponentTags` (`|MakeArray` _output_get_2) _returnvalue_3)))
  (`KismetSystemLibrary.Delay` 5.0)
  (`self.Select_empty`))

(event `Select_empty`
  (bind (_output_mesh _output_fuel _output_active _output_placed) (break `/Game/structures/S_fuel` (`|GetArrayItem` (`self.Fuels`) (`self.index`))))
  (`KismetSystemLibrary.Delay` 15.0)
  (set `self.index` (`KismetMathLibrary.RandomIntegerInRange` 0 (- (`KismetArrayLibrary.Array_Length` (`self.Fuels`)) 1)))
  (`PrimitiveComponent.SetMaterial` _output_mesh 0 "/AnimationSharing/AnimSharingRed.AnimSharingRed")
  (`KismetArrayLibrary.Array_Set` (`self.Fuels`) (`self.index`) (make `/Game/structures/S_fuel` _output_mesh 0.0 false _output_placed))
  (`/Game/bps/bp_reactor_main.ED_Recalculate_Power_Event` (`self.Bp_reactor_main`))
  (`KismetSystemLibrary.Delay` (`KismetMathLibrary.RandomFloatInRange` 50.0 60.0))
  (`self.Select_empty`))

(event `self.Cube.OnComponentBeginOverlap`
  (params (OverlappedComponent :type "PrimitiveComponent Object Reference") (OtherActor :type "Actor Object Reference") (OtherComp :type "PrimitiveComponent Object Reference") (OtherBodyIndex :type Integer) (bFromSweep :type Boolean) (SweepResult :type "HitResult Structure (by ref)"))
  (bind (_returnvalue_x _returnvalue_y _returnvalue_z) (`KismetMathLibrary.BreakVector` (`SceneComponent.K2_GetComponentLocation` (`self.DefaultSceneRoot`))))
  (bind _returnvalue (+ _returnvalue_x -200.0))
  (for (_array_element _array_index) (`ActorComponent.ComponentTags` OtherComp)
    (if (== _array_index 0)
      (set `self.ind_to_remove` (`KismetStringLibrary.Conv_NameToString` _array_element))))
  (`KismetArrayLibrary.Array_Remove` (`self.Fuels`) (`KismetStringLibrary.Conv_StringToInt` (`self.ind_to_remove`)))
  (`ActorComponent.K2_DestroyComponent` OtherComp)
  (bind _returnvalue_2 (`AddComponent|NODE_AddStaticMeshComponent-1` :`RelativeTransform` (`KismetMathLibrary.MakeTransform` (`KismetMathLibrary.MakeVector` _returnvalue) (struct) (0.5 0.5 0.5))))
  (`SceneComponent.K2_SetWorldLocation` _returnvalue_2 (`KismetMathLibrary.MakeVector` _returnvalue (+ _returnvalue_y 100.0) _returnvalue_z) false false)
  (`StaticMeshComponent.SetStaticMesh` _returnvalue_2 "/Engine/BasicShapes/Cube.Cube")
  (`PrimitiveComponent.SetSimulatePhysics` _returnvalue_2 true)
  (`PrimitiveComponent.SetMaterial` _returnvalue_2 0 "/AnimationSharing/AnimSharingGreen.AnimSharingGreen")
  (bind _returnvalue_3 (`KismetArrayLibrary.Array_Add` (`self.Fuels`) (make `/Game/structures/S_fuel` _returnvalue_2 100.0 true)))
  (bind _output_get (set `self.ind` (`KismetStringLibrary.Conv_IntToString` _returnvalue_3)))
  (bind _output_get_2 (set `self.tag` (`KismetStringLibrary.Conv_StringToName` _output_get)))
  (set `ActorComponent.ComponentTags` (`|MakeArray` _output_get_2) _returnvalue_2))

(event `self.Cube1.OnComponentBeginOverlap`
  (params (OverlappedComponent :type "PrimitiveComponent Object Reference") (OtherActor :type "Actor Object Reference") (OtherComp :type "PrimitiveComponent Object Reference") (OtherBodyIndex :type Integer) (bFromSweep :type Boolean) (SweepResult :type "HitResult Structure (by ref)"))
  (bind _output_get (set `self.Component Tags` (`ActorComponent.ComponentTags` OtherComp)))
  (for (_array_element _array_index) _output_get
    (if (== _array_index 0)
      (bind _output_get_2 (set `self.ind_aa` (`KismetStringLibrary.Conv_NameToString` _array_element)))
      (bind _output_get_3 (set `self.Array` (`|MakeArray` (`KismetStringLibrary.Conv_StringToName` _output_get_2) "Placed")))
      (set `ActorComponent.ComponentTags` _output_get_3 OtherComp)))
  (for (_array_element_2 _array_index_2) (`self.Fuels`)
    (if (`ActorComponent.ComponentHasTag` (break `/Game/structures/S_fuel` _array_element_2) "Placed")
      (`KismetArrayLibrary.Array_Set` (`self.Fuels`) _array_index_2 (make `/Game/structures/S_fuel` (break `/Game/structures/S_fuel` _array_element_2) (`.Fuel_5_EA564127436107125587148396CBF3D6` (break `/Game/structures/S_fuel` _array_element_2)) (`.active_9_DDA82008483E56247C1AD5A378F9DDC9` (break `/Game/structures/S_fuel` _array_element_2)) true))))
  (`/Game/bps/bp_reactor_main.ED_Recalculate_Power_Event` (`self.Bp_reactor_main`)))

(event `self.Cube1.OnComponentEndOverlap`
  (params (OverlappedComponent :type "PrimitiveComponent Object Reference") (OtherActor :type "Actor Object Reference") (OtherComp :type "PrimitiveComponent Object Reference") (OtherBodyIndex :type Integer))
  (bind _output_get (set `self.Component Tags` (`ActorComponent.ComponentTags` OtherComp)))
  (for (_array_element _array_index) _output_get
    (if (== _array_index 0)
      (bind _output_get_2 (set `self.ind_aa` (`KismetStringLibrary.Conv_NameToString` _array_element)))
      (bind _output_get_3 (set `self.Array` (`|MakeArray` _array_element "notPlaced")))
      (set `ActorComponent.ComponentTags` _output_get_3 OtherComp)))
  (for (_array_element_2 _array_index_2) (`self.Fuels`)
    (if (`ActorComponent.ComponentHasTag` (break `/Game/structures/S_fuel` _array_element_2) "notPlaced")
      (`KismetArrayLibrary.Array_Set` (`self.Fuels`) _array_index_2 (make `/Game/structures/S_fuel` (break `/Game/structures/S_fuel` _array_element_2) (`.Fuel_5_EA564127436107125587148396CBF3D6` (break `/Game/structures/S_fuel` _array_element_2)) (`.active_9_DDA82008483E56247C1AD5A378F9DDC9` (break `/Game/structures/S_fuel` _array_element_2))))))
  (`/Game/bps/bp_reactor_main.ED_Recalculate_Power_Event` (`self.Bp_reactor_main`)))

(fn `UserConstructionScript`)