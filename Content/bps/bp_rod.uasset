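; Reactor rod actor with three selectable states, Full, Half and No, that set its PowerLos value for the reactor.
; BeginPlay finds and caches the Bp_reactor_main actor in the level.
; ED_Select_rod_Event reads HoldingCompoment, highlights the matching component by swapping active and inactive materials, and updates PowerLos.
; Each valid selection then calls the reactor's EDRecalculatePowerEvent to recompute power.
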(event `self.ReceiveBeginPlay`
  (bind _returnvalue (`GameplayStatics.GetActorOfClass` "/Game/bps/bp_reactor_main.bp_reactor_main_C"))
  (set `self.bp_reactor_main` _returnvalue))

(event `ED_Select_rod_Event`
  (if (`KismetStringLibrary.EqualEqual_StrStr` (`self.holding_compoment`) "Full")
    (`PrimitiveComponent.SetMaterial` (`self.Full`) 0 (`self.active_mat`))
    (`PrimitiveComponent.SetMaterial` (`self.Half`) 0 (`self.non_active_mat`))
    (`PrimitiveComponent.SetMaterial` (`self.No`) 0 (`self.non_active_mat`))
    (set `self.power_los` 100.0)
    (`/Game/bps/bp_reactor_main.ED_Recalculate_Power_Event` (`self.bp_reactor_main`) :!label _label)
    (elif (`KismetStringLibrary.EqualEqual_StrStr` (`self.holding_compoment`) "Half")
      (`PrimitiveComponent.SetMaterial` (`self.Full`) 0 (`self.non_active_mat`))
      (`PrimitiveComponent.SetMaterial` (`self.Half`) 0 (`self.active_mat`))
      (`PrimitiveComponent.SetMaterial` (`self.No`) 0 (`self.non_active_mat`))
      (set `self.power_los` 50.0)
      (goto _label)
      (elif (`KismetStringLibrary.EqualEqual_StrStr` (`self.holding_compoment`) "No")
        (`PrimitiveComponent.SetMaterial` (`self.Full`) 0 (`self.non_active_mat`))
        (`PrimitiveComponent.SetMaterial` (`self.Half`) 0 (`self.non_active_mat`))
        (`PrimitiveComponent.SetMaterial` (`self.No`) 0 (`self.active_mat`))
        (set `self.power_los` 0.0)
        (goto _label)))))

(fn `UserConstructionScript`)