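; Water valve wheel actor that feeds water into the main reactor and signals water danger.
; On BeginPlay it finds the reactor actor and spawns a warning light beside itself.
; Each tick it toggles that light from the reactor's WaterDanger flag.
; While Active, it adds WaterInput to the reactor's water every frame, unscaled by delta time, and spins the valve mesh.
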(event `self.ReceiveBeginPlay`
  (bind _returnvalue (`GameplayStatics.GetActorOfClass` "/Game/bps/bp_reactor_main.bp_reactor_main_C"))
  (set `self.bp_reactor_main` _returnvalue)
  (bind _returnvalue_2 (`|SpawnActorFromClass` "/Game/bps/bp_warning_light.bp_warning_light_C" (`KismetMathLibrary.MakeTransform` (+ (`SceneComponent.K2_GetComponentLocation` (`self.DefaultSceneRoot`)) (-100.0 90.0 50.0)) (struct :`Roll` -90.0)) "Undefined" "MultiplyWithRoot" null null))
  (set `self.bp_warning_light` _returnvalue_2))

(event `self.ReceiveTick`
  (params (DeltaSeconds :type "Float (single-precision)"))
  (bind _bp_reactor_main (`self.bp_reactor_main`))
  (bind _bp_warning_light (`self.bp_warning_light`))
  (if (`/Game/bps/bp_reactor_main.water_danger` (`self.bp_reactor_main`))
    (`/Game/bps/bp_warning_light.warning_light_on` _bp_warning_light)
    (else
      (`/Game/bps/bp_warning_light.warning_light_off` _bp_warning_light)))
  (if (`self.active`)
    (set `/Game/bps/bp_reactor_main.water` (+ (`/Game/bps/bp_reactor_main.water` _bp_reactor_main) (`self.water_input`)) _bp_reactor_main)
    (set `self.rotation` (+ (* DeltaSeconds 5.0) (`self.rotation`)))
    (`SceneComponent.K2_SetWorldRotation` (`self.valve_test`) (`KismetMathLibrary.MakeRotator` 90.0 (`self.rotation`)) false false)))

(fn `UserConstructionScript`)