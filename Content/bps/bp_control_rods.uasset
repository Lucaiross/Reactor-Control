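; Control rod bank actor that reduces the main reactor's power.
; On BeginPlay it caches the reactor actor, then spawns a row of eight Bp_rod actors spaced along Y from its root and stores them in an array.
; A recalculate-loss event sums each rod's power loss and subtracts the total from the reactor's current Power.
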(event `self.ReceiveBeginPlay`
  (bind (_returnvalue_x _returnvalue_y _returnvalue_z) (`KismetMathLibrary.BreakVector` (`SceneComponent.K2_GetComponentLocation` (`self.DefaultSceneRoot`))))
  (bind _returnvalue (`GameplayStatics.GetActorOfClass` "/Game/bps/bp_reactor_main.bp_reactor_main_C"))
  (set `self.bp_reactor_main` _returnvalue)
  (for _index (range 8)
    (bind _returnvalue_2 (`|SpawnActorFromClass` "/Game/bps/bp_rod.bp_rod_C" (`KismetMathLibrary.MakeTransform` (`KismetMathLibrary.MakeVector` _returnvalue_x (+ (* _index 50) _returnvalue_y) _returnvalue_z)) "Undefined" "MultiplyWithRoot" null null))
    (bind _output_get (set `self.bp_rod` _returnvalue_2))
    (`KismetArrayLibrary.Array_Add` (`self.Array`) _output_get)))

(event `ED_recalulate_loss_Event`
  (bind _bp_reactor_main (`self.bp_reactor_main`))
  (set `self.power_down` 0.0)
  (for _array_element (`self.Array`)
    (set `self.power_down` (+ (`self.power_down`) (`/Game/bps/bp_rod.power_los` _array_element))))
  (set `/Game/bps/bp_reactor_main.power` (- (`/Game/bps/bp_reactor_main.power` _bp_reactor_main) (`self.power_down`)) _bp_reactor_main))

(fn `UserConstructionScript`)