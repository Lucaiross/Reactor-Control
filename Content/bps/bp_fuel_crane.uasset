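; Player-operated fuel crane that moves along X and Y and uses a hook to pick up and drop fuel.
; A selection event maps the held component's name to a button, which Tick acts on while Active.
; Timelines sweep the hook down, attaching any bp_fuel component it hits, then raise it toward its starting height.
; Triggering the hook while loaded releases the fuel into physics, with a DoOnce and timeline gating the reset.
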(event `self.ReceiveBeginPlay`
  (bind (_returnvalue_x _returnvalue_y _returnvalue_z) (`KismetMathLibrary.BreakVector` (`SceneComponent.K2_GetComponentLocation` (`self.Hook_crane`))))
  (set `self.z_default` _returnvalue_z)
  (bind _returnvalue (`GameplayStatics.GetActorOfClass` "/Game/bps/bp_reactor_main.bp_reactor_main_C"))
  (set `self.bp_reactor_main` _returnvalue)
  (bind _returnvalue_2 (`GameplayStatics.GetActorOfClass` "/Game/bps/bp_fuel.bp_fuel_C"))
  (set `self.bp_fuel` _returnvalue_2))

(event `self.ReceiveTick`
  (params (DeltaSeconds :type "Float (single-precision)"))
  (bind (_returnvalue_x _returnvalue_y _returnvalue_z) (`KismetMathLibrary.BreakVector` (`SceneComponent.K2_GetComponentLocation` (`self.Second_crane`))))
  (bind (_returnvalue_x_2 _returnvalue_y_2 _returnvalue_z_2) (`KismetMathLibrary.BreakVector` (`SceneComponent.K2_GetComponentLocation` (`self.Main_crane`))))
  (bind (_returnvalue_x_3 _returnvalue_y_3 _returnvalue_z_3) (`KismetMathLibrary.BreakVector` (`SceneComponent.K2_GetComponentLocation` (`self.Main_crane`))))
  (bind (_returnvalue_x_4 _returnvalue_y_4 _returnvalue_z_4) (`KismetMathLibrary.BreakVector` (`SceneComponent.K2_GetComponentLocation` (`self.Second_crane`))))
  (if (`self.Active`)
    (switch `int` (`self.button`)
      (:`0`
        (`SceneComponent.K2_SetWorldLocation` (`self.Main_crane`) (`KismetMathLibrary.MakeVector` (- _returnvalue_x_2 (`self.x_speed_crane`)) _returnvalue_y_2 _returnvalue_z_2) false false))
      (:`1`
        (`SceneComponent.K2_SetWorldLocation` (`self.Main_crane`) (`KismetMathLibrary.MakeVector` (+ _returnvalue_x_3 (`self.x_speed_crane`)) _returnvalue_y_3 _returnvalue_z_3) false false))
      (:`2`
        (`SceneComponent.K2_SetWorldLocation` (`self.Second_crane`) (`KismetMathLibrary.MakeVector` _returnvalue_x_4 (- _returnvalue_y_4 (`self.y_speed_crane`)) _returnvalue_z_4) false false))
      (:`3`
        (`SceneComponent.K2_SetWorldLocation` (`self.Second_crane`) (`KismetMathLibrary.MakeVector` _returnvalue_x (+ _returnvalue_y (`self.y_speed_crane`)) _returnvalue_z) false false))
      (:`4`
        (`self.TryHook`)))))

(event `TryHook`
  (bind _hook_crane (`self.Hook_crane`))
  (bind _z_default (`self.z_default`))
  (bind _sweep_hit_result_hit_component (`self.Sweep Hit Result Hit Component`))
  (bind (_returnvalue_x _returnvalue_y _returnvalue_z) (`KismetMathLibrary.BreakVector` (`SceneComponent.K2_GetComponentLocation` (`self.Hook_crane`))))
  (bind (_returnvalue_x_2 _returnvalue_y_2 _returnvalue_z_2) (`KismetMathLibrary.BreakVector` (`SceneComponent.K2_GetComponentLocation` (`self.Hook_crane`))))
  (bind _returnvalue (+ _returnvalue_z (`self.z_speed`)))
  (if (`self.fuel_grabbed`)
    (`/Engine/EditorBlueprintResources/StandardMacros.DoOnce` false :!label _label
      (:`Completed`
        (`SceneComponent.K2_DetachFromComponent` _sweep_hit_result_hit_component "KeepWorld" "KeepWorld" "KeepWorld" false)
        (`PrimitiveComponent.SetSimulatePhysics` _sweep_hit_result_hit_component true)
        (`Timeline|Timeline_1` :!via `PlayFromStart`
          (:`Finished`
            (set `self.fuel_grabbed` false)
            (goto _label :!via `Reset`)))))
    (else
      (`Timeline|Timeline` :!via `PlayFromStart`
        (:`Update`
          (bind _sweephitresult (`SceneComponent.K2_SetWorldLocation` (`self.Hook_crane`) (`KismetMathLibrary.MakeVector` _returnvalue_x_2 _returnvalue_y_2 (- _returnvalue_z_2 (`self.z_speed`))) true false))
          (cast `/Game/bps/bp_fuel` (`.HitActor` (`GameplayStatics.BreakHitResult` _sweephitresult)))
          (if (`GameplayStatics.BreakHitResult` _sweephitresult)
            (`SceneComponent.K2_AttachToComponent` (`.HitComponent` (`GameplayStatics.BreakHitResult` _sweephitresult)) (`self.Hook_crane`) "None" "KeepWorld" "KeepWorld" "KeepWorld" true)
            (set `self.fuel_grabbed` true)
            (set `self.Sweep Hit Result Hit Component` (`.HitComponent` (`GameplayStatics.BreakHitResult` _sweephitresult)))))
        (:`Finished`
          (`Timeline|Timeline_0` :!via `PlayFromStart`
            (:`Update`
              (if (> _z_default _returnvalue)
                (`SceneComponent.K2_SetWorldLocation` _hook_crane (`KismetMathLibrary.MakeVector` _returnvalue_x _returnvalue_y _returnvalue) true false)
                (else
                  (`SceneComponent.K2_SetWorldLocation` _hook_crane (`KismetMathLibrary.MakeVector` _returnvalue_x _returnvalue_y _z_default) true false))))))))))

(event `ED_Fuel_crane_selection_Event`
  (if (`KismetStringLibrary.EqualEqual_StrStr` (`self.holding_component`) "Left")
    (set `self.button` 0)
    (elif (`KismetStringLibrary.EqualEqual_StrStr` (`self.holding_component`) "Right")
      (set `self.button` 1)
      (elif (`KismetStringLibrary.EqualEqual_StrStr` (`self.holding_component`) "Forward")
        (set `self.button` 2)
        (elif (`KismetStringLibrary.EqualEqual_StrStr` (`self.holding_component`) "Back")
          (set `self.button` 3)
          (elif (`KismetStringLibrary.EqualEqual_StrStr` (`self.holding_component`) "Hook")
            (set `self.button` 4)))))))

(fn `UserConstructionScript`)